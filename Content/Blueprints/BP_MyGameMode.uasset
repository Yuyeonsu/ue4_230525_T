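; Game mode that keeps spawning BP_Light actors in the level and sets an Exploding flag based on their count.
; BeginPlay shows the PlayerUI_Light widget and starts a looping timer that spawns lights at random horizontal positions in a square area at fixed height.
; Tick counts all BP_Light actors every frame and sets Exploding to true when the count exactly equals PassedLighits.
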(event `self.ReceiveBeginPlay`
  (bind _returnvalue (`|CreateWidget` "/Game/UMG/PlayerUI_Light.PlayerUI_Light_C"))
  (`UserWidget.AddToViewport` _returnvalue 0)
  (`KismetSystemLibrary.K2_SetTimerDelegate` (delegate `커스텀이벤트_0`) 3.0 true))

(event `커스텀이벤트_0`
  (`|SpawnActorFromClass` "/Game/Blueprints/BP_Light.BP_Light_C" (`KismetMathLibrary.MakeTransform` (`KismetMathLibrary.MakeVector` (`KismetMathLibrary.RandomFloatInRange` -940.0 940.0) (`KismetMathLibrary.RandomFloatInRange` -940.0 940.0) 50.0) (struct)) "Undefined" "OverrideRootScale" null null))

(event `self.ReceiveTick`
  (params (DeltaSeconds :type "Float (single-precision)"))
  (bind _outactors (`GameplayStatics.GetAllActorsOfClass` "/Game/Blueprints/BP_Light.BP_Light_C"))
  (bind _output_get (set `self.NumberOfLights` (`KismetArrayLibrary.Array_Length` _outactors)))
  (if (== _output_get (`self.PassedLighits`))
    (set `self.Exploding` true)))

(fn `UserConstructionScript`)